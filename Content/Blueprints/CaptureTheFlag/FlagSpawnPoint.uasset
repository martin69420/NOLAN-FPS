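; Team flag spawn point for Capture the Flag that doubles as the team's capture zone.
; On BeginPlay it spawns a Flag with its team and itself as parent, only in the CaptureTheFlag game mode.
; When a same-team flag carrier overlaps CaptureRadius, a TeamData table lookup confirms the carried flag is an enemy's.
; A capture clears and destroys the carried flag, then adds one team point through FirstPersonGameState.
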(event OnComponentBeginOverlap(CaptureRadius)
  (params (OverlappedComponent :type Primitive%20Component%20Object%20Reference) (OtherActor :type Actor%20Object%20Reference) (OtherComp :type Primitive%20Component%20Object%20Reference) (OtherBodyIndex :type Integer) (bFromSweep :type Boolean) (SweepResult :type Hit%20Result%20Structure%20%28by%20ref%29))
  (CallFunction|TryCapture OtherActor))

(event Custom|SpawnFlag
  (if (== (Utilities|GetClass (Game|GetGameMode)) "/Game/FirstPersonBP/FirstPerson/Gamemodes/CaptureTheFlag.CaptureTheFlag_C")
    (Game|SpawnActorfromClass "/Game/Blueprints/CaptureTheFlag/Flag.Flag_C" (Transformation|GetActorTransform) "Undefined" 0 (Variables|Default|GetTeam) self 0)))

(event Custom|TryCapture
  (params (Character :type Actor%20Object%20Reference))
  (bind _team (Variables|Default|GetTeam))
  (bind _asfirst_person_character (Utilities|Casting|CastToFirstPersonCharacter Character))
  (if (and (Variables|/Game/FirstPersonBP/Character/FirstPersonCharacter.FirstPersonCharacter_C|GetIsHoldingFlag? _asfirst_person_character) (Utilities|Enum|Equal(Enum) (Variables|/Game/FirstPersonBP/Character/FirstPersonCharacter.FirstPersonCharacter_C|GetTeam _asfirst_person_character) _team))
    (bind _returnvalue (Utilities|GetDataTableRow "/Game/FirstPersonBP/FirstPerson/Team/TeamData.TeamData" (Utilities|String|StringToName (Utilities|String|EnumtoString (Variables|/Game/Blueprints/CaptureTheFlag/Flag.Flag_C|GetTeam (Variables|/Game/FirstPersonBP/Character/FirstPersonCharacter.FirstPersonCharacter_C|GetFlagRef _asfirst_person_character)))))
      (:then
        (if (Utilities|Array|ContainsItem (.EnemyTeams (Utilities|Struct|BreakTeamStruct _returnvalue)) (Utilities|String|EnumtoString _team))
          (CallFunction|Capture _asfirst_person_character))))))

(event Custom|Capture
  (params (Character :type First%20Person%20Character%20Object%20Reference))
  (Variables|/Game/FirstPersonBP/Character/FirstPersonCharacter.FirstPersonCharacter_C|SetIsHoldingFlag? Character false)
  (Default|Destroy (Variables|/Game/FirstPersonBP/Character/FirstPersonCharacter.FirstPersonCharacter_C|GetFlagRef Character))
  (Variables|/Game/FirstPersonBP/Character/FirstPersonCharacter.FirstPersonCharacter_C|SetFlagRef Character 0)
  (bind _asfirst_person_game_state (Utilities|Casting|CastToFirstPersonGameState (Game|GetGameState)))
  (Default|AddTeamScore _asfirst_person_game_state (Variables|/Game/FirstPersonBP/Character/FirstPersonCharacter.FirstPersonCharacter_C|GetTeam Character) 1))

(event EventBeginPlay
  (CallFunction|SpawnFlag))

(fn ConstructionScript)