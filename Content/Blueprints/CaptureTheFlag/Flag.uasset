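; Capture-the-flag flag actor, coloured by team from a data table, with a matching marker widget.
; Characters whose team lists the flag's team as an enemy pick it up on overlap, attaching it to their flag point.
; The carrier's death event drops it and starts a despawn timer, cleared on pickup.
; On expiry, the flag asks its parent to spawn a replacement, then destroys itself.
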(event OnComponentBeginOverlap(SphereCollision)
  (params (OverlappedComponent :type Primitive%20Component%20Object%20Reference) (OtherActor :type Actor%20Object%20Reference) (OtherComp :type Primitive%20Component%20Object%20Reference) (OtherBodyIndex :type Integer) (bFromSweep :type Boolean) (SweepResult :type Hit%20Result%20Structure%20%28by%20ref%29))
  (CallFunction|AttemptPickup OtherActor))

(event Custom|AttemptPickup
  (params (Actor :type Actor%20Object%20Reference))
  (if (not (Variables|Default|GetIsAttached?))
    (bind _asfirst_person_character (Utilities|Casting|CastToFirstPersonCharacter Actor))
    (bind _returnvalue (Utilities|GetDataTableRow "/Game/FirstPersonBP/FirstPerson/Team/TeamData.TeamData" (Utilities|String|StringToName (Utilities|String|EnumtoString (Variables|/Game/FirstPersonBP/Character/FirstPersonCharacter.FirstPersonCharacter_C|GetTeam _asfirst_person_character))))
      (:then
        (if (Utilities|Array|ContainsItem (.EnemyTeams (Utilities|Struct|BreakTeamStruct _returnvalue)) (Utilities|String|EnumtoString (Variables|Default|GetTeam)))
          (CallFunction|AttachtoPlayer _asfirst_person_character))))))

(event Custom|AttachToPlayer
  (params (Character :type First%20Person%20Character%20Object%20Reference))
  (Transformation|AttachComponentToComponent (Variables|/Game/FirstPersonBP/Character/FirstPersonCharacter.FirstPersonCharacter_C|GetCTF_FlagPoint Character) "None" "SnapToTarget" "SnapToTarget" "KeepRelative" true)
  (Variables|/Game/FirstPersonBP/Character/FirstPersonCharacter.FirstPersonCharacter_C|SetFlagRef Character self)
  (Variables|/Game/FirstPersonBP/Character/FirstPersonCharacter.FirstPersonCharacter_C|SetIsHoldingFlag? Character true)
  (EventDispatchers|BindEventtoPlayerDead Character (delegate Custom|DropFlag))
  (Variables|Default|SetIsAttached? true)
  (CallFunction|ClearDespawnTimer))

(event Custom|BeginDespawnTimer
  (bind _returnvalue (Utilities|Time|SetTimerbyEvent (delegate Custom|Destroy) 0.0 false (Variables|Default|GetDespawnTimer))))

(event Custom|DropFlag
  (params (Controller :type First%20Person%20Controller%20Object%20Reference) (Character :type First%20Person%20Character%20Object%20Reference))
  (CallFunction|BeginDespawnTimer)
  (Transformation|DetachFromActor "KeepRelative" "KeepRelative" "KeepRelative")
  (Variables|Default|SetIsAttached? false)
  (Variables|/Game/FirstPersonBP/Character/FirstPersonCharacter.FirstPersonCharacter_C|SetIsHoldingFlag? Character false)
  (Variables|/Game/FirstPersonBP/Character/FirstPersonCharacter.FirstPersonCharacter_C|SetFlagRef Character 0))

(event Custom|Destroy
  (Default|SpawnFlag (Variables|Default|GetParent))
  (Actor|DestroyActor))

(event Custom|SetColour
  (bind _returnvalue (Utilities|GetDataTableRow "/Game/FirstPersonBP/FirstPerson/Team/TeamData.TeamData" (Utilities|String|StringToName (Utilities|String|EnumtoString (Variables|Default|GetTeam))))
    (:then
      (bind _returnvalue_2 (Rendering|Material|CreateDynamicMaterialInstance (Variables|Default|GetSphere) 0 "/Game/Materials/TeamMaterial_Inst.TeamMaterial_Inst" "Team" :!class /Script/Engine.PrimitiveComponent))
      (Rendering|Material|SetVectorParameterValue _returnvalue_2 "BaseColour" (.Colour (Utilities|Struct|BreakTeamStruct _returnvalue)) :!class /Script/Engine.MaterialInstanceDynamic)
      (Default|SetTeam (.AsUI%20Flag%20Marker (Utilities|Casting|CastToUI_FlagMarker (UserInterface|GetWidget (Variables|Default|GetWidget)))) (Variables|Default|GetTeam)))))

(event Custom|ClearDespawnTimer
  (Utilities|Time|ClearandInvalidateTimerbyHandle (stale Custom|BeginDespawnTimer _returnvalue)))

(event EventBeginPlay
  (CallFunction|SetColour))

(fn ConstructionScript)