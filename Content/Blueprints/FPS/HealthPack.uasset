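; A health pickup for the FPS character that heals on sphere overlap and respawns after a short delay.
; It triggers only when the overlapping FirstPersonCharacter is below max health, healing by applying negative damage and playing a slurp sound.
; A DoOnce guards the pickup while it is hidden with collision off, then resets when it reappears.
; Tick spins the cube around its yaw axis.
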(event OnComponentBeginOverlap(Sphere)
  (params (OverlappedComponent :type Primitive%20Component%20Object%20Reference) (OtherActor :type Actor%20Object%20Reference) (OtherComp :type Primitive%20Component%20Object%20Reference) (OtherBodyIndex :type Integer) (bFromSweep :type Boolean) (SweepResult :type Hit%20Result%20Structure%20%28by%20ref%29))
  (bind _asfirst_person_character (Utilities|Casting|CastToFirstPersonCharacter OtherActor))
  (if (< (Variables|/Game/FirstPersonBP/Character/FirstPersonCharacter.FirstPersonCharacter_C|GetHealth _asfirst_person_character) (Variables|/Game/FirstPersonBP/Character/FirstPersonCharacter.FirstPersonCharacter_C|GetMaxHealth _asfirst_person_character))
    (Utilities|FlowControl|DoOnce false :!label _label
      (:Completed
        (Game|Damage|ApplyDamage OtherActor -5e+01 0 0)
        (Audio|PlaySoundatLocation "/Game/SFX/HealthSlurp.HealthSlurp" (Transformation|GetActorLocation) "0, 0, 0" 0.5 1.0 0.0 0 0 0)
        (Rendering|SetActorHiddenInGame true)
        (Collision|SetActorEnableCollision false)
        (Utilities|FlowControl|Delay 7.0)
        (Rendering|SetActorHiddenInGame false)
        (Collision|SetActorEnableCollision true)
        (goto _label Reset)))))

(event EventTick
  (params (DeltaSeconds :type Float%20%28single-precision%29))
  (Transformation|AddRelativeRotation (Variables|Default|GetCube) (Math|Rotator|MakeRotator 0.0 0.0 (* DeltaSeconds 1e+02)) false false))

(fn ConstructionScript)