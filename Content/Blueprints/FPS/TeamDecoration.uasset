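; TeamDecoration is a team-coloured cube decoration that only remains in Deathmatch matches where its team is in play.
; The cube takes its Scale in the construction script and again at BeginPlay.
; At BeginPlay it also looks up its Team in the TeamData table and applies that colour through a dynamic material instance.
; It then destroys itself if the Deathmatch game mode is not team-based or disallows that team, but stays under other game modes.
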(event Custom|SetScale
  (Transformation|SetWorldScale3D (Variables|Default|GetCube) (Variables|Default|GetScale)))

(event Custom|AttemptDestroy
  (bind _asdeathmatch (Utilities|Casting|CastToDeathmatch (Game|GetGameMode)))
  (if (not (and (Variables|/Game/FirstPersonBP/FirstPerson/Gamemodes/Deathmatch.Deathmatch_C|GetTeamGamemode? _asdeathmatch) (Utilities|Array|ContainsItem (Variables|/Game/FirstPersonBP/FirstPerson/Gamemodes/Deathmatch.Deathmatch_C|GetAllowedTeams _asdeathmatch) (Variables|Default|GetTeam))))
    (Actor|DestroyActor)))

(event Custom|SetColour
  (bind _returnvalue (Utilities|GetDataTableRow "/Game/FirstPersonBP/FirstPerson/Team/TeamData.TeamData" (Utilities|String|StringToName (Utilities|String|EnumtoString (Variables|Default|GetTeam))))
    (:then
      (bind _returnvalue_2 (Rendering|Material|CreateDynamicMaterialInstance (Variables|Default|GetCube) 0 "/Game/Materials/TeamMaterial_Inst.TeamMaterial_Inst" "Team" :!class /Script/Engine.PrimitiveComponent))
      (Rendering|Material|SetVectorParameterValue _returnvalue_2 "BaseColour" (.Colour (Utilities|Struct|BreakTeamStruct _returnvalue)) :!class /Script/Engine.MaterialInstanceDynamic))))

(event EventBeginPlay
  (CallFunction|SetScale)
  (CallFunction|SetColour)
  (CallFunction|AttemptDestroy))

(fn ConstructionScript
  (Transformation|SetWorldScale3D (Variables|Default|GetCube) (Variables|Default|GetScale)))